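; Save object for the player farming system that stores arrays of per-level and per-player save data structs.
; Level and player records are looked up by linear search on name, and updates overwrite the matching entry or append a new one.
; Level records can also be removed by name or built as new structs from a level name, which are returned without being stored.
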(fn CurrentLevelSaveData
  (params (LevelName :type String))
  ;[1 1 1] Returns the level save data for a level name
  (bind (_returnvalue _levelsavedata) (Saving|FindLevelSaveData LevelName))
  (if _returnvalue
    (return _levelsavedata)
    (else
      (return ""))))

(fn UpdateLevelSaveData
  (params (LevelSaveData :type S%20Level%20Save%20Data%20Structure))
  ;[1 1 1] Loop though the level save data and find the level save data with the same name and set the new level data, if no matching name found create new level save data in level save data array
  (for (_array_element _array_index) (Variables|Default|GetLevelSaveData)
    (LocalVariables|SetSaveIndexL _array_index)
    (if (Utilities|Enum|Equal(Enum) (.LevelName (Utilities|Struct|BreakS_LevelSaveData _array_element)) (.LevelName (Utilities|Struct|BreakS_LevelSaveData LevelSaveData)))
      (Utilities|Array|SetArrayElem (Variables|Default|GetLevelSaveData) (LocalVariables|GetSaveIndexL) LevelSaveData true)
      (return)))
  (Utilities|Array|Add (Variables|Default|GetLevelSaveData) LevelSaveData)
  (return))

(fn ClearLevelSaveData
  (params (LevelName :type String))
  ;[1 1 1] Search for level name in level save data and remove it
  (for (_array_element _array_index) (Variables|Default|GetLevelSaveData)
    (if (Utilities|Enum|Equal(Enum) (.LevelName (Utilities|Struct|BreakS_LevelSaveData _array_element)) LevelName)
      (Utilities|Array|RemoveIndex (Variables|Default|GetLevelSaveData) _array_index))))

(fn CreateLevelSaveData
  (params (LevelName :type String))
  ;[1 1 1] Create new level save data
  (bind _structout (Utilities|Struct|SetmembersinS_LevelSaveData (LocalVariables|GetTempLevelSaveDataL) LevelName))
  (return _structout))

(fn FindLevelSaveData
  (params (LevelName :type String))
  ;[1 1 1] Search for level save data using level name
  (for _array_element (Variables|Default|GetLevelSaveData)
    (if (Utilities|Enum|Equal(Enum) (Utilities|Struct|BreakS_LevelSaveData _array_element) LevelName)
      (return true _array_element)))
  (return false ""))

(fn UpdatePlayerSaveData
  (params (PlayerSaveData :type S%20Player%20Save%20Data%20Structure))
  ;[1 1 1] Finds and update player save data with new input data, if not found a new player save data is added
  (for (_array_element _array_index) (Variables|Default|GetPlayerSaveData)
    (LocalVariables|SetIndexL _array_index)
    (if (Utilities|Enum|Equal(Enum) (.PlayerName (Utilities|Struct|BreakS_PlayerSaveData _array_element)) (.PlayerName (Utilities|Struct|BreakS_PlayerSaveData PlayerSaveData)))
      (Utilities|Array|SetArrayElem (Variables|Default|GetPlayerSaveData) (LocalVariables|GetIndexL) PlayerSaveData)
      (return)))
  (Utilities|Array|Add (Variables|Default|GetPlayerSaveData) PlayerSaveData))

(fn FindPlayerSaveData
  (params (PlayerName :type String))
  ;[1 1 1] Find player save data using player name
  (for _array_element (Variables|Default|GetPlayerSaveData)
    (LocalVariables|SetPlayerSaveDataL _array_element)
    (if (Utilities|Enum|Equal(Enum) (.PlayerName (Utilities|Struct|BreakS_PlayerSaveData _array_element)) PlayerName)
      (return true (LocalVariables|GetPlayerSaveDataL))))
  (return false ""))