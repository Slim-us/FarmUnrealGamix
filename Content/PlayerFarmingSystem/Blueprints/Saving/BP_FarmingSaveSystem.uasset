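; Server-side save system for the player farming system that saves and restores planters, plants and tools per level.
; It registers with the game mode, can load on BeginPlay and runs an optional looping autosave.
; Saving rebuilds the current level's record, collects data from BP_FarmingSaveInterface actors and writes the slot asynchronously.
; Loading pauses autosave, notifies those actors, then respawns saved objects by class and transform.
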(fn ConstructionScript)

(fn AutoSave
  ;[1 1 1] If saver run the Server Save Game event using the current save name
  (Networking|SwitchHasAuthority
    (:Authority
      (CallFunction|ServerSaveGame (Variables|LoadSettings|GetSaveName)))))

(fn StartAutoSaveTimer
  ;[1 1 1] If Use Auto Save is true start timer to run AutoSave function
  (if (Variables|AutoSave|GetUseAutoSave)
    (if (not (Utilities|Time|IsValidTimerHandle (Variables|DoNotEdit|GetAutoSaveTimer)))
      (bind _returnvalue (Utilities|Time|SetTimerbyFunctionName 0 "AutoSave" (Variables|AutoSave|GetAutoSaveTime) true))
      (Variables|DoNotEdit|SetAutoSaveTimer _returnvalue))))

(fn DebugText
  (params (InString :type String) (TextColor :type Linear%20Color%20Structure :default "(R=0.000000,G=1.000000,B=0.000000,A=1.000000)") (Duration :type Float%20%28double-precision%29))
  (bind _debugmode (Variables|Debug|GetDebugMode))
  ;[1 1 1] If debug mode is true print text
  (Development|PrintString InString _debugmode _debugmode TextColor Duration))

(fn LoadTool
  (params (ToolSaveData :type S%20Tool%20Save%20Data%20Structure))
  (bind (_class _transform) (Utilities|Struct|BreakS_ToolSaveData ToolSaveData))
  ;[1 1 1] Spawn actor using Class from ToolSaveData, run SetLoadedbySave event and toggle the tool on or off using enabled value from save
  (bind _returnvalue (Game|SpawnActorfromClass _class _transform "Undefined" 0 0))
  (bind _output_get (LocalVariables|SetNewActorL _returnvalue))
  (Class|BPFarmingSaveInterface|PFSSetLoadedbySave(Message) _output_get true)
  (Class|BPFarmingInteractionInterface|PFSToggleOn/Off(Message) (LocalVariables|GetNewActorL) (.Enabled (Utilities|Struct|BreakS_ToolSaveData ToolSaveData))))

(fn LoadPlanter
  (params (PlanterSaveData :type S%20Planter%20Save%20Data%20Structure))
  (bind (_class _transform) (Utilities|Struct|BreakS_PlanterSaveData PlanterSaveData))
  ;[1 1 1] Spawn actor from PlanterSaveData then loop though the planters saved plants and run the load plant function using that data
  (bind _returnvalue (Game|SpawnActorfromClass _class _transform "Undefined" 0 0))
  (bind _output_get (LocalVariables|SetNewActorL _returnvalue))
  (Class|BPFarmingSaveInterface|PFSLoadAttachedPlants(Message) _output_get PlanterSaveData))

(fn LoadPlant
  (params (PlantSaveData :type S%20Plant%20Save%20Data%20Structure) (AttachActor :type Actor%20Object%20Reference))
  (bind (_class _transform) (Utilities|Struct|BreakS_PlantSaveData PlantSaveData))
  ;[1 1 1] Spawn actor using the Class from the Plant Save Data and run the SetLoadedbySave event
  (bind _returnvalue (Game|SpawnActorfromClass _class _transform "Undefined" 0 0))
  (LocalVariables|SetNewActorL _returnvalue)
  ;[1 1 1] Get the plant's plant component
  (bind _plantcomponent (Class|BPFarmingPlantInterface|PFSPlantComponent(Message) (LocalVariables|GetNewActorL)))
  (Utilities|IsValid _plantcomponent
    (:Is%20Valid
      (bind _output_get (LocalVariables|SetPlantComponentL _plantcomponent))
      ;[1 1 1] Loads plant save data
      (Default|LoadPlantSaveData _output_get PlantSaveData AttachActor))))

(fn SelectSaveSlot
  (params (SaveName :type String))
  ;[1 1 1] Checks if the save name input is valid, if not use the save systems current save name
  (if (Utilities|Enum|Equal(Enum) SaveName "")
    (return (Variables|LoadSettings|GetSaveName))
    (else
      (return SaveName))))

(fn FindPlayerSave
  (params (PlayerName :type String))
  ;[1 1 1] Finds the player save data using the players name
  (bind _returnvalue (SaveGame|DoesSaveGameExist (Variables|LoadSettings|GetSaveName)))
  (if _returnvalue
    (bind _returnvalue_2 (SaveGame|LoadGamefromSlot (Variables|LoadSettings|GetSaveName)))
    (bind _asbp_farming_save_object (Utilities|Casting|CastToBP_FarmingSaveObject _returnvalue_2))
    (bind (_returnvalue_3 _playersavedata) (Default|FindPlayerSaveData _asbp_farming_save_object PlayerName))
    (return _returnvalue_3 _playersavedata)
    (else
      (return false ""))))

(event EventBeginPlay
  ;[1 1 1] On begin play set the save system in the game mode and start the auto save timer, if load on begin play then call the load save game event
  (Networking|SwitchHasAuthority
    (:Authority
      (Class|BPFarmingGameModeInterface|PFSSetSaveSystem(Message) (Game|GetGameMode) self)
      (Saving|StartAutoSaveTimer)
      (bind _returnvalue (Game|GetCurrentLevelName true))
      (Variables|DoNotEdit|SetCurrentLevel _returnvalue)
      (if (Variables|LoadSettings|GetLoadSaveOnBeginPlay)
        (CallFunction|ServerLoadGame (Variables|LoadSettings|GetSaveName))))))

(event Custom|ServerSaveGame
  (params (SaveName :type String))
  ;[1 1 1] Runs the code to save the game
  (|CreateSaveData SaveName)
  (|SaveActorData)
  (|AsyncSaveGametoSlot (Variables|DoNotEdit|GetSaveGameData) (Variables|DoNotEdit|GetSavingSlotName)
    (:Completed
      (Variables|DoNotEdit|SetSaving false)
      (Debug|DebugText "Save Complete" "(R=0.000000,G=1.000000,B=0.000000,A=1.000000)" 2.0))))

(event Custom|ServerLoadGame
  (params (SaveName :type String))
  ;[1 1 1] Runs the code to load a save game
  (|LoadSaveData SaveName)
  (|CurrentActorsLoadCall)
  (|LoadSaveGameActors))

(event Custom|DeleteSaveGame
  ;[1 1 1] Run to delete the current save name file
  (|DeleteSave))