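; Potato plant Blueprint for the player farming system, providing destruction meshes for the crop's growth stages.
; AddDestructionMesh compares the plant component's current static mesh against the seedling, two later growth stages and the fully grown vegetable mesh.
; A match adds a Geometry Collection component at identity transform, so the mesh itself serves as the growth-stage indicator.
; The construction script only calls its parent.
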(fn ConstructionScript
  (|CallParentFunction))

(fn AddDestructionMesh
  ;[1 0 0] Add destruction mesh for growth stage 1
  (if (== (Variables|/Game/PlayerFarmingSystem/Blueprints/Components/BP_PlantComponent.BP_PlantComponent_C|GetStaticMesh (Variables|Default|GetBP_PlantComponent)) "/Game/PlayerFarmingSystem/Meshes/Static/SM_Seedling_04.SM_Seedling_04")
    (AddComponent|AddGeometryCollectionComponent false (Math|Transform|MakeTransform "0, 0, 0"))
    (else
      ;[1 0 0] Add destruction mesh for growth stage 2
      (if (== (Variables|/Game/PlayerFarmingSystem/Blueprints/Components/BP_PlantComponent.BP_PlantComponent_C|GetStaticMesh (Variables|Default|GetBP_PlantComponent)) "/Game/PlayerFarmingSystem/Meshes/Static/SM_PotatoPlant_02.SM_PotatoPlant_02")
        (AddComponent|AddGeometryCollectionComponent false (Math|Transform|MakeTransform "0, 0, 0"))
        (else
          ;[1 0 0] Add destruction mesh for growth stage 3
          (if (== (Variables|/Game/PlayerFarmingSystem/Blueprints/Components/BP_PlantComponent.BP_PlantComponent_C|GetStaticMesh (Variables|Default|GetBP_PlantComponent)) "/Game/PlayerFarmingSystem/Meshes/Static/SM_PotatoPlant_01.SM_PotatoPlant_01")
            (AddComponent|AddGeometryCollectionComponent false (Math|Transform|MakeTransform "0, 0, 0"))
            (else
              ;[1 0 0] Add destruction mesh for vegetables grown
              (if (== (Variables|/Game/PlayerFarmingSystem/Blueprints/Components/BP_PlantComponent.BP_PlantComponent_C|GetStaticMesh (Variables|Default|GetBP_PlantComponent)) "/Game/PlayerFarmingSystem/Meshes/Static/SM_PotatoPlant_03.SM_PotatoPlant_03")
                (AddComponent|AddGeometryCollectionComponent false (Math|Transform|MakeTransform "0, 0, 0"))))))))))