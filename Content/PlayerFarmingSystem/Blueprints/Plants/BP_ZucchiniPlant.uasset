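; BP_ZucchiniPlant is the zucchini plant Blueprint in the player farming system, supplying destruction meshes for each growth stage.
; AddDestructionMesh compares the BPPlantComponent static mesh against four stage meshes, from early growth through vegetables grown.
; A match adds a Geometry Collection component at the default relative transform.
; The construction script only calls its parent.
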(fn ConstructionScript
  (|CallParentFunction))

(fn AddDestructionMesh
  ;[1 0 0] Add destruction mesh for growth stage 1
  (if (== (Variables|/Game/PlayerFarmingSystem/Blueprints/Components/BP_PlantComponent.BP_PlantComponent_C|GetStaticMesh (Variables|Default|GetBP_PlantComponent)) "/Game/PlayerFarmingSystem/Meshes/Static/SM_ZucchiniPlant_01.SM_ZucchiniPlant_01")
    (AddComponent|AddGeometryCollectionComponent false (Math|Transform|MakeTransform "0, 0, 0"))
    (else
      ;[1 0 0] Add destruction mesh for growth stage 2
      (if (== (Variables|/Game/PlayerFarmingSystem/Blueprints/Components/BP_PlantComponent.BP_PlantComponent_C|GetStaticMesh (Variables|Default|GetBP_PlantComponent)) "/Game/PlayerFarmingSystem/Meshes/Static/SM_ZucchiniPlant_02.SM_ZucchiniPlant_02")
        (AddComponent|AddGeometryCollectionComponent false (Math|Transform|MakeTransform "0, 0, 0"))
        (else
          ;[1 0 0] Add destruction mesh for growth stage 3
          (if (== (Variables|/Game/PlayerFarmingSystem/Blueprints/Components/BP_PlantComponent.BP_PlantComponent_C|GetStaticMesh (Variables|Default|GetBP_PlantComponent)) "/Game/PlayerFarmingSystem/Meshes/Static/SM_ZucchiniPlant_03.SM_ZucchiniPlant_03")
            (AddComponent|AddGeometryCollectionComponent false (Math|Transform|MakeTransform "0, 0, 0"))
            (else
              ;[1 0 0] Add destruction mesh for vegetables grown
              (if (== (Variables|/Game/PlayerFarmingSystem/Blueprints/Components/BP_PlantComponent.BP_PlantComponent_C|GetStaticMesh (Variables|Default|GetBP_PlantComponent)) "/Game/PlayerFarmingSystem/Meshes/Static/SM_ZucchiniPlant_04.SM_ZucchiniPlant_04")
                (AddComponent|AddGeometryCollectionComponent false (Math|Transform|MakeTransform "0, 0, 0"))))))))))