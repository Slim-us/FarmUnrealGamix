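; Base plant actor for the player farming system, exposing its plant component, info panel widget and socket requirement.
; On save, placed plants that are neither previews nor attached write component stats into the current level's save data.
; Meshes ignore the preview channel to prevent placement on plants, while a multicast-managed box blocks placement while a dead plant awaits respawn.
; Preview plants can show at grow-effect start scale, applied one tick after BeginPlay.
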(fn ConstructionScript)

(fn PFSRequireSocket
  (return (Variables|FarmingSettings|Sockets|GetRequireSocket)))

(fn SavePlantData
  (params (SaveData :type BP%20Farming%20Save%20Object%20Object%20Reference))
  ;[1 1 1] Find level save data using current level name
  (bind _returnvalue (Game|GetCurrentLevelName true))
  (bind _levelsavedata (Default|CurrentLevelSaveData SaveData _returnvalue))
  (LocalVariables|SetLevelSaveDataL _levelsavedata)
  ;[1 1 1] Gets all plant stats and sets them in plant save data
  (bind _plantsavedata (Default|SetPlantSaveData (Variables|Default|GetBP_PlantComponent)))
  ;[1 1 1] Add plant save data to the level save data and update the save data object with the new level save data
  (Utilities|Array|Add (Utilities|Struct|BreakS_LevelSaveData (LocalVariables|GetLevelSaveDataL)) _plantsavedata)
  (Default|UpdateLevelSaveData SaveData (LocalVariables|GetLevelSaveDataL)))

(fn AddPlaceholderCollision
  ;[1 1 1] Adds placeholder collision for when the plant is not visible during respawn
  (Utilities|IsValid (Variables|Collision|GetPlaceholderCollision)
    (:Is%20Valid
      (Components|DestroyComponent (Variables|Collision|GetPlaceholderCollision)))
    (:Is%20Not%20Valid
      _))
  (bind _returnvalue (AddComponent|AddBoxComponent false (Math|Transform|MakeTransform "0, 0, 0")))
  (bind _output_get (Variables|Collision|SetPlaceholderCollision _returnvalue))
  (Collision|SetCollisionResponsetoAllChannels _output_get "ECR_Ignore")
  (Collision|SetCollisionResponsetoChannel _output_get (Variables|FarmingSettings|Collision|GetPlacementCollisionChannel) "ECR_Block"))

(fn PFSWidget
  (return "/Game/PlayerFarmingSystem/Blueprints/Widgets/BP_PlantInfoPanel.BP_PlantInfoPanel_C"))

(fn SetupCollision
  ;[1 1 1] Sets meshes to ignore the preview channel to stop placement on plants
  (bind _output_get (LocalVariables|SetPrimitiveComponentsL (Actor|GetComponentsByClass "/Script/Engine.PrimitiveComponent")))
  (for _array_element _output_get
    (if (not (Components|ComponentHasTag _array_element "IgnoreMesh"))
      (Collision|SetCollisionResponsetoChannel _array_element (Variables|FarmingSettings|Collision|GetPreviewCollisionChannel) "ECR_Ignore"))))

(fn StartGrowEffectScale
  (bind _bp_plantcomponent (Variables|Default|GetBP_PlantComponent))
  (bind _bp_plantcomponent_2 (Variables|Default|GetBP_PlantComponent))
  (bind _groweffectstartscale (Variables|/Game/PlayerFarmingSystem/Blueprints/Components/BP_PlantComponent.BP_PlantComponent_C|GetGrowEffectStartScale _bp_plantcomponent))
  (bind _groweffectstartscale_2 (Variables|/Game/PlayerFarmingSystem/Blueprints/Components/BP_PlantComponent.BP_PlantComponent_C|GetGrowEffectStartScale _bp_plantcomponent_2))
  ;[1 1 1] If using grow effect and use scale for preview set the meshes scale
  (if (Variables|/Game/PlayerFarmingSystem/Blueprints/Components/BP_PlantComponent.BP_PlantComponent_C|GetUseGrowEffect (Variables|Default|GetBP_PlantComponent))
    (if (Variables|FarmingSettings|Preview|GetUseGrowEffectGrowthScaleForPreview)
      ;[1 1 1] Sets the scale of the meshes to the row effect start scale
      (for _array_element (Actor|GetComponentsByClass "/Script/Engine.StaticMeshComponent")
        (Utilities|IsValid _array_element
          (:Is%20Valid
            (if (not (Components|ComponentHasTag _array_element "IgnoreMesh"))
              (Transformation|SetWorldScale3D _array_element (Math|Vector|MakeVector _groweffectstartscale _groweffectstartscale _groweffectstartscale))))))
      (for _array_element_2 (Actor|GetComponentsByClass "/Script/Engine.SkeletalMeshComponent")
        (Utilities|IsValid _array_element_2
          (:Is%20Valid
            (if (not (Components|ComponentHasTag _array_element_2 "IgnoreMesh"))
              (Transformation|SetWorldScale3D _array_element_2 (Math|Vector|MakeVector _groweffectstartscale_2 _groweffectstartscale_2 _groweffectstartscale_2)))))))))

(event EventPFSSaveActor
  (params (SaveObject :type BP%20Farming%20Save%20Object%20Object%20Reference))
  ;[1 1 1] Runs when the game saves, to store the plants data in the save game object
  (Utilities|IsPreview?
    (:false
      (Utilities|IsAttached?
        (:False
          (Saving|SavePlantData SaveObject))))))

(event Custom|MulticastAddPlaceholderCollision
  ;[1 1 1] On placeholder collision add collision
  (Collision|AddPlaceholderCollision))

(event Custom|MulticastRemovePlaceholderCollision
  (bind _placeholdercollision (Variables|Collision|GetPlaceholderCollision))
  ;[1 1 1] Removes the placeholder collision
  (Utilities|IsValid _placeholdercollision
    (:Is%20Valid
      (Components|DestroyComponent _placeholdercollision))))

(event EventPFSRemovePlaceholderCollision
  ;[1 1 1] Removes the placeholder collision
  (CallFunction|MulticastRemovePlaceholderCollision))

(event EventPFSAddPlaceholderCollision
  ;[1 1 1] On placeholder collision add collision
  (CallFunction|MulticastAddPlaceholderCollision))

(event EventBeginPlay
  ;[1 1 1] On begin play if health is 0 add placeholder collision
  (|CallParentFunction)
  (Collision|SetupCollision)
  (Utilities|FlowControl|Sequence
    (:then_0
      (if (<= (Variables|/Game/PlayerFarmingSystem/Blueprints/Components/BP_PlantComponent.BP_PlantComponent_C|GetHealth (Variables|Default|GetBP_PlantComponent)) 0.0)
        (Collision|AddPlaceholderCollision)))
    (:then_1
      ;[1 1 1] Sets the preview scale
      (Utilities|FlowControl|DelayUntilNextTick)
      (Utilities|IsPreview?
        (:true
          (Preview|StartGrowEffectScale))))))

(fn PFSPlantComponent
  (return (Variables|Default|GetBP_PlantComponent)))