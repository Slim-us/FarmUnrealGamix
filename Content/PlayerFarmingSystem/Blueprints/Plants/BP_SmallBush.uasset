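; BP_SmallBush is a small bush plant in the player farming system that supports destruction at its growth stages.
; AddDestructionMesh compares the plant component's static mesh against the seedling, small plant and grown plant meshes, then adds a Geometry Collection component at an identity relative transform for the matching stage.
; The construction script only calls its parent, and nothing in this file calls AddDestructionMesh.
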(fn ConstructionScript
  (|CallParentFunction))

(fn AddDestructionMesh
  ;[1 0 0] Add destruction mesh for growth stage 1
  (if (== (Variables|/Game/PlayerFarmingSystem/Blueprints/Components/BP_PlantComponent.BP_PlantComponent_C|GetStaticMesh (Variables|Default|GetBP_PlantComponent)) "/Game/PlayerFarmingSystem/Meshes/Static/SM_Seedling_01.SM_Seedling_01")
    (AddComponent|AddGeometryCollectionComponent false (Math|Transform|MakeTransform "0, 0, 0"))
    (else
      ;[1 0 0] Add destruction mesh for growth stage 2
      (if (== (Variables|/Game/PlayerFarmingSystem/Blueprints/Components/BP_PlantComponent.BP_PlantComponent_C|GetStaticMesh (Variables|Default|GetBP_PlantComponent)) "/Game/PlayerFarmingSystem/Meshes/Static/SM_SmallPlant_01.SM_SmallPlant_01")
        (AddComponent|AddGeometryCollectionComponent false (Math|Transform|MakeTransform "0, 0, 0"))
        (else
          ;[1 0 0] Add destruction mesh for growth stage 2
          (if (== (Variables|/Game/PlayerFarmingSystem/Blueprints/Components/BP_PlantComponent.BP_PlantComponent_C|GetStaticMesh (Variables|Default|GetBP_PlantComponent)) "/Game/PlayerFarmingSystem/Meshes/Static/SM_GrownPlant_01.SM_GrownPlant_01")
            (AddComponent|AddGeometryCollectionComponent false (Math|Transform|MakeTransform "0, 0, 0"))))))))