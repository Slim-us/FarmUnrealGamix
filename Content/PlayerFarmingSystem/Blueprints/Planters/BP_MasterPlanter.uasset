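; BP_MasterPlanter is the planter actor in the player farming system, handling save and load of itself and its attached plants.
; On save, non-preview planters pack their class, transform and data from attached BP_MasterPlant children's plant components into the current level's save data.
; On load, it spawns each saved plant and passes the saved data and itself as attach actor to the plant component.
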(fn ConstructionScript)

(fn SavePlanterData
  (params (SaveData :type BP%20Farming%20Save%20Object%20Object%20Reference))
  ;[1 1 1] Gets current level data from the save data
  (bind _returnvalue (Game|GetCurrentLevelName true))
  (bind _levelsavedata (Default|CurrentLevelSaveData SaveData _returnvalue))
  (LocalVariables|SetLevelSaveDataL _levelsavedata)
  ;[1 1 1] Get planter save info and sets it to a planter save data struct
  (bind _plantersavedata (Saving|SetPlanterSaveData))
  ;[1 1 1] Add the planter save data to the level save data then set the level save data in the save data object
  (Utilities|Array|Add (Utilities|Struct|BreakS_LevelSaveData (LocalVariables|GetLevelSaveDataL)) _plantersavedata)
  (Default|UpdateLevelSaveData SaveData (LocalVariables|GetLevelSaveDataL)))

(fn SetPlanterSaveData
  ;[1 1 1] Gets the attached plant save data and planter save data and sets it to a planter save data struct ready for saving
  (bind _plantsavedata (Saving|PreparePlantSaveData))
  (bind _structout (Utilities|Struct|SetmembersinS_PlanterSaveData (LocalVariables|GetPlanterSaveDataL) (Utilities|GetClass self) (Transformation|GetActorTransform) _plantsavedata))
  (return _structout))

(fn LoadAttachedPlants
  (params (PlanterSaveData :type S%20Planter%20Save%20Data%20Structure))
  (for _array_element (.Plants (Utilities|Struct|BreakS_PlanterSaveData PlanterSaveData))
    (bind _returnvalue (Game|SpawnActorfromClass (.Class (Utilities|Struct|BreakS_PlantSaveData _array_element)) (.Transform (Utilities|Struct|BreakS_PlantSaveData _array_element)) "AlwaysSpawn" self 0))
    (bind _plantcomponent (Class|BPFarmingPlantInterface|PFSPlantComponent(Message) _returnvalue))
    (Utilities|IsValid _plantcomponent
      (:Is%20Valid
        (Default|LoadPlantSaveData _plantcomponent _array_element self)))))

(fn PreparePlantSaveData
  ;[1 1 1] Loops though the attached plants and gets there plant variables to add them to the plant save data
  (bind _output_get (LocalVariables|SetAttachedActorsL (Actor|GetAttachedActors true false)))
  (for _array_element _output_get
    (LocalVariables|SetActorL _array_element)
    (if (Utilities|ClassIsChildOf (Utilities|GetClass _array_element) "/Game/PlayerFarmingSystem/Blueprints/Plants/BP_MasterPlant.BP_MasterPlant_C")
      (bind _plantcomponent (Class|BPFarmingPlantInterface|PFSPlantComponent(Message) (LocalVariables|GetActorL)))
      (bind _output_get_2 (LocalVariables|SetPlantComponentL _plantcomponent))
      (bind _plantsavedata (Default|SetPlantSaveData _output_get_2))
      (Utilities|Array|Add (LocalVariables|GetPlantSaveDataL) _plantsavedata)))
  (return (LocalVariables|GetPlantSaveDataL)))

(event EventPFSLoadAttachedPlants
  (params (PlanterSaveData :type S%20Planter%20Save%20Data%20Structure))
  ;[1 1 1] Loads the attached plants
  (Saving|LoadAttachedPlants PlanterSaveData))

(event EventPFSSaveActor
  (params (SaveObject :type BP%20Farming%20Save%20Object%20Object%20Reference))
  ;[1 1 1] Saves the planter data to the save game
  (if (not (CallFunction|GetPreview))
    (Saving|SavePlanterData SaveObject)))