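; Game mode for the player farming system that spawns players from saved data and exposes shared farming state.
; The SpawnDefaultPawnAtTransform override names each player by player count, finds or spawns BP_FarmingSaveSystem, then spawns the pawn at its saved transform and restores farming resources.
; Without load-on-begin-play or a matching save, the given start transform is used.
; Interface functions expose the save system and relay night, rain and directional lights through BPFarmingGameModeComponent.
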(fn ConstructionScript)

(fn SpawnDefaultPawnatTransform
  (params (NewPlayer :type Controller%20Object%20Reference) (SpawnTransform :type Transform%20%28by%20ref%29))
  ;[1 1 1] Set player name
  (Class|GameModeBase|ChangeName NewPlayer (Utilities|String|ToString(Integer) (Utilities|Array|Length (Variables|/Script/Engine.GameStateBase|GetPlayerArray (Game|GetGameState)))) false)
  ;[1 1 1] Get reference to save system, if none spawn save system
  (Utilities|IsValid (Variables|Saving|GetSaveSystem)
    (:Is%20Valid
      _)
    (:Is%20Not%20Valid
      (bind _outactors (Actor|GetAllActorsOfClass "/Game/PlayerFarmingSystem/Blueprints/Saving/BP_FarmingSaveSystem.BP_FarmingSaveSystem_C"))
      (if (Utilities|Array|IsValidIndex _outactors)
        (bind _output_get (Variables|Saving|SetSaveSystem (Utilities|Array|Get(acopy) _outactors)))
        (Utilities|IsValid _output_get
          (:Is%20Valid
            _)
          (:Is%20Not%20Valid
            (bind _returnvalue (Game|SpawnActorfromClass "/Game/PlayerFarmingSystem/Blueprints/Saving/BP_FarmingSaveSystem.BP_FarmingSaveSystem_C" (Math|Transform|MakeTransform "0, 0, 0" "0, 0, 0" "1.000000,1.000000,1.000000") "Undefined" 0 0 :!label _label))
            (Variables|Saving|SetSaveSystem _returnvalue)))
        (else
          (goto _label)))))
  ;[1 1 1] Load player location from save, if no save then use player start location
  (if (Variables|/Game/PlayerFarmingSystem/Blueprints/Saving/BP_FarmingSaveSystem.BP_FarmingSaveSystem_C|GetLoadSaveOnBeginPlay (Variables|Saving|GetSaveSystem))
    (bind (_returnvalue_2 _playersavedata) (Default|FindPlayerSave (Variables|Saving|GetSaveSystem) (PlayerState|GetPlayerName (Variables|/Script/Engine.Controller|GetPlayerState NewPlayer))))
    (if _returnvalue_2
      (bind _output_get_2 (LocalVariables|SetPlayerSaveDataL _playersavedata))
      (bind _returnvalue_3 (Game|SpawnActorfromClass (Variables|Default|GetDefaultPawnClass) (Utilities|Struct|BreakS_PlayerSaveData _output_get_2) "Undefined" NewPlayer 0))
      (LocalVariables|SetNewCharacterL _returnvalue_3)
      ;[1 1 1] Set resources from player save data
      (Variables|/Game/PlayerFarmingSystem/Blueprints/Components/BP_PlayerFarmingComponent.BP_PlayerFarmingComponent_C|SetResources (Actor|GetComponentbyClass NewPlayer "/Game/PlayerFarmingSystem/Blueprints/Components/BP_PlayerFarmingComponent.BP_PlayerFarmingComponent_C") (Utilities|Struct|BreakS_PlayerSaveData (LocalVariables|GetPlayerSaveDataL)))
      (return (LocalVariables|GetNewCharacterL))
      (else
        _)))
  (bind _returnvalue_4 (Game|SpawnActorfromClass (Variables|Default|GetDefaultPawnClass) SpawnTransform "Undefined" NewPlayer 0))
  (return _returnvalue_4))

(event EventPFSSetSaveSystem
  (params (SaveSystem :type BP%20Farming%20Save%20System%20Object%20Reference))
  ;[1 1 1] Set SaveSystem
  (Variables|Saving|SetSaveSystem SaveSystem))

(event EventPGSSetIsNight
  (params (IsNight :type Boolean))
  ;[1 1 1] Set IsNight
  (Default|SetIsNight (Variables|Default|GetBP_FarmingGameModeComponent) IsNight))

(event EventPFSSetIsRaining
  (params (IsRaining :type Boolean) (RainAmount :type Float%20%28double-precision%29))
  ;[1 1 1] Set IsNight
  (Default|SetIsRaining (Variables|Default|GetBP_FarmingGameModeComponent) IsRaining RainAmount))

(fn PFSGetDirectionalLights
  (return (Variables|/Game/PlayerFarmingSystem/Blueprints/Components/BP_FarmingGameModeComponent.BP_FarmingGameModeComponent_C|GetDirectionalLights (Variables|Default|GetBP_FarmingGameModeComponent))))

(fn PFSGetFarmingGameModeComponent
  (return (Variables|Default|GetBP_FarmingGameModeComponent)))

(fn PFSGetIsNight
  (return (Variables|/Game/PlayerFarmingSystem/Blueprints/Components/BP_FarmingGameModeComponent.BP_FarmingGameModeComponent_C|GetIsNight (Variables|Default|GetBP_FarmingGameModeComponent))))

(fn PFSGetIsRaining
  (bind _bp_farminggamemodecomponent (Variables|Default|GetBP_FarmingGameModeComponent))
  (return (Variables|/Game/PlayerFarmingSystem/Blueprints/Components/BP_FarmingGameModeComponent.BP_FarmingGameModeComponent_C|GetIsRaining _bp_farminggamemodecomponent) (Variables|/Game/PlayerFarmingSystem/Blueprints/Components/BP_FarmingGameModeComponent.BP_FarmingGameModeComponent_C|GetRainAmount _bp_farminggamemodecomponent)))

(fn PFSGetSaveSystem
  (return (Variables|Saving|GetSaveSystem)))