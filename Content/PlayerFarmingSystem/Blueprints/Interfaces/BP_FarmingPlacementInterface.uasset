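; Blueprint interface for placeable objects in the Player Farming System, defining the contract between placement logic and farming actors.
; It exposes preview state, farming type, ground-detect components and placement collision for positioning and validating an object.
; Socket queries report whether an object uses or requires sockets and which ones it allows.
; Demolish, Pickup and Placed functions cover the object's lifecycle, with Pickup returning whether pickup is possible.
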(fn PFSGetPreview
  (return false))

(fn PFSSetPreview
  (params (Preview :type Boolean))
  (return))

(fn PFSFarmingType
  (return "NewEnumerator0"))

(fn PFSGetGroundDetectComponents
  (return 0))

(fn PFSPlacementCollision
  (return 0))

(fn PFSUseSockets
  (return false))

(fn PFSRequireSocket
  (return false))

(fn PFSAllowedSockets
  (return "NewEnumerator0"))

(fn PFSDemolish)

(fn PFSPickup
  (return false 0))

(fn PFSPlaced)