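; Blueprint interface for the game mode in the Player Farming System, exposing shared farming world state to other objects.
; It declares getters and setters for the save system, night state, and rain state with a rain amount.
; It also declares getters for directional lights and the farming game mode component.
; The functions are empty declarations, so implementers supply the behavior.
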(fn PFSGetSaveSystem
  (return 0))

(fn PFSSetSaveSystem
  (params (SaveSystem :type BP%20Farming%20Save%20System%20Object%20Reference)))

(fn PFSGetDirectionalLights
  (return 0))

(fn PFSGetIsNight
  (return false))

(fn PGSSetIsNight
  (params (IsNight :type Boolean))
  (return))

(fn PFSGetIsRaining
  (return false 0.0))

(fn PFSSetIsRaining
  (params (IsRaining :type Boolean) (RainAmount :type Float%20%28single-precision%29)))

(fn PFSGetFarmingGameModeComponent
  (return 0))