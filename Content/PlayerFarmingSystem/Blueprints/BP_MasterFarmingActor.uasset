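; Base actor for placeable farming objects, exposing preview, socket, pickup, save and placement data through PFS functions.
; On BeginPlay it caches ground-detect and collision components, then non-preview instances drop placement collision and ignore the light channel.
; Destruction breaks child-supplied Geometry Collections, with optional timed removal, and destroys attached plants, as does demolishing.
; Placement plays a multicast sound, and the load event destroys the actor.
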(fn ConstructionScript)

(fn DestroyFarmingPlacementCollision
  ;[1 1 1] Destroy placement collision
  (for _array_element (Variables|DoNotEdit|GetPlacementCollision)
    (Utilities|IsValid _array_element
      (:Is%20Valid
        (Components|DestroyComponent _array_element)))))

(fn AddDestructionMesh
  ;[1 1 1] Override in child blueprints
)

(fn StartDestructionMeshTimer
  (params (RemoveTime :type Float%20%28double-precision%29))
  ;[1 1 1] Remove current destruction mesh components, restart remove destruction mesh component timer and then create new destruction mesh function
  (Destruction|RemoveDestructionMesh)
  (Utilities|FlowControl|Sequence
    (:then_0
      (if (> RemoveTime 0.0)
        (Utilities|Time|SetTimerbyFunctionName 0 "RemoveDestructionMesh" RemoveTime)))
    (:then_1
      (Destruction|AddDestructionMesh)
      (Destruction|BreakDestructionMeshes)
      (Destruction|DestroyAttachedActors)
      (Destruction|DestructionEffect))))

(fn RemoveDestructionMesh
  ;[1 1 1] Destroy all destruction component
  (Components|DestroyComponent (Actor|GetComponentsByClass "/Script/GeometryCollectionEngine.GeometryCollectionComponent")))

(fn DestroyAttachedActors
  ;[1 1 1] Get all attached actors and destroy them
  (bind _output_get (LocalVariables|SetAttachedActorsL (Actor|GetAttachedActors true false)))
  (for _array_element _output_get
    (Utilities|IsValid _array_element
      (:Is%20Valid
        (if (Utilities|ClassIsChildOf (Utilities|GetClass _array_element) "/Game/PlayerFarmingSystem/Blueprints/Plants/BP_MasterPlant.BP_MasterPlant_C")
          (Actor|DestroyActor _array_element))))))

(fn UpdateComponents
  ;[1 1 1] Get and set the components
  (Variables|DoNotEdit|SetGroundDetectComponents (Actor|GetComponentsByClass "/Game/PlayerFarmingSystem/Blueprints/Components/BP_GroundDetectComponent.BP_GroundDetectComponent_C"))
  (Variables|DoNotEdit|SetPlacementCollision (Actor|GetComponentsbyTag "/Script/Engine.PrimitiveComponent" "Collision")))

(fn DestructionMeshCollision
  (params (Component :type Primitive%20Component%20Object%20Reference))
  ;[1 1 1] Sets the plants destruction mesh to ignore everything that isnt a static or dynamic object to avoid interfering with other collision
  (Collision|SetCollisionResponsetoAllChannels Component "ECR_Ignore")
  (Collision|SetCollisionResponsetoChannel Component "ECC_WorldStatic" "ECR_Block")
  (Collision|SetCollisionResponsetoChannel Component "ECC_WorldDynamic" "ECR_Block"))

(fn BreakDestructionMeshes
  ;[1 1 1] Loops though the destruction meshes and breaks them
  (bind _output_get (LocalVariables|SetDestructionMeshesL (Actor|GetComponentsByClass "/Script/GeometryCollectionEngine.GeometryCollectionComponent")))
  (for _array_element _output_get
    (bind _output_get_2 (LocalVariables|SetDestructionComponentL _array_element))
    (Utilities|IsValid _output_get_2
      (:Is%20Valid
        (Destruction|DestructionMeshCollision (LocalVariables|GetDestructionComponentL))
        ;[1 1 1] Break destruction mesh
        (Class|GeometryCollectionComponent|ApplyKinematicField (LocalVariables|GetDestructionComponentL) 9999.0 (Physics|GetCenterOfMass (LocalVariables|GetDestructionComponentL) "None"))))))

(fn DestructionEffect
  ;[1 1 1] Used in child blueprints
)

(fn GetPreview
  (return (Variables|DoNotEdit|GetPreview)))

(event EventBeginPlay
  ;[1 1 1] On begin play set components array and if not preview removes the build preview collision
  (|CallParentFunction)
  (Components|UpdateComponents)
  (Utilities|FlowControl|DelayUntilNextTick)
  (Utilities|IsPreview?
    (:false
      (Collision|DestroyFarmingPlacementCollision)
      ;[1 1 1] Sets plants to ignore light channel, this stops plants blocking light from others and self
      (for _array_element (Actor|GetComponentsByClass "/Script/Engine.PrimitiveComponent")
        (Collision|SetCollisionResponsetoChannel _array_element (Variables|FarmingSettings|Collision|GetLightCollisionChannel) "ECR_Ignore")))))

(event EventPFSSetPreview
  (params (Preview :type Boolean))
  ;[1 1 1] On Set Preview update the preview variable
  (Variables|DoNotEdit|SetPreview Preview))

(event EventPFSPlaced
  ;[1 1 1] On Set Preview update the preview variable
  (CallFunction|MulticastPlaceSound))

(event EventPFSLoadActor
  (params (SaveData :type BP%20Farming%20Save%20Object%20Object%20Reference))
  ;[1 1 1] On load actor destroy actor
  (Actor|DestroyActor))

(event EventPFSSetLoadedbySave
  (params (LoadedBySave :type Boolean))
  ;[1 1 1] On Set loaded by save update the variable
  (Variables|DoNotEdit|SetLoadedBySave LoadedBySave))

(event EventPFSDemolish
  ;[1 1 1] On demolish destroy attached actors and destroy actor
  (Destruction|DestroyAttachedActors)
  (Actor|DestroyActor))

(event Custom|MulticastPlaceSound
  ;[1 1 1] Play place sound
  (Audio|PlaySoundatLocation (Variables|FarmingSettings|GetPlaceSound) (Transformation|GetActorLocation) "0, 0, 0" 1.0 1.0 0.0 0 0 0 0))

(fn PFSAllowedSockets
  (return (Variables|FarmingSettings|Sockets|GetSocketTypes)))

(fn PFSFarmingType
  (bind _farmingdetails (Variables|FarmingSettings|GetFarmingDetails))
  (bind _rowname (Utilities|Struct|BreakDataTableRowHandle _farmingdetails))
  (bind (_returnvalue _details) (CallFunction|PFSFarmingActorDetails _rowname))
  (if _returnvalue
    (return (.FarmingType (Utilities|Struct|BreakS_FarmingActorDetails _details)))))

(fn PFSGetGroundDetectComponents
  (return (Variables|DoNotEdit|GetGroundDetectComponents)))

(fn PFSGetLoadedbySave
  (return (Variables|DoNotEdit|GetLoadedBySave)))

(fn PFSGetPreview
  ;[1 1 1] Is Preview?
  (return (Preview|GetPreview)))

(fn PFSPickup
  ;[1 1 1] Returns the can pickup and resources
  (return (Variables|FarmingSettings|Pickup|GetCanPickup) (Variables|FarmingSettings|Pickup|GetPickupResources)))

(fn PFSPlacementCollision
  (return (Variables|DoNotEdit|GetPlacementCollision)))

(fn PFSRequireSocket
  (return false))

(fn PFSUseSockets
  (return (Variables|FarmingSettings|Sockets|GetUseSockets)))

(fn PFSWidget
  (return 0))