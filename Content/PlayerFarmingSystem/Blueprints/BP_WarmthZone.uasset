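; BP_WarmthZone is a box-volume actor in the player farming system that supplies a warmth effect to plants inside it.
; On the server, BeginPlay registers overlapping plants and binds to the game mode farming component's update event, rescanning after a short random delay when the reported location falls inside the box.
; Scans briefly enable box collision, add the zone to new plants' WarmthZones and update their warmth.
; An interface function exposes Enabled and Warmth.
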(fn ConstructionScript)

(fn UpdateOverlappingPlantsWarmth
  ;[1 1 1] Loop though plants within area and add self to plants warmth zone
  (Collision|SetCollisionEnabled (Variables|Default|GetBox) "QueryOnly")
  (bind _outactors (Collision|ComponentOverlapActors (Variables|Default|GetBox) (Transformation|GetWorldTransform (Variables|Default|GetBox)) (Utilities|Array|MakeArray "ObjectTypeQuery2") "/Game/PlayerFarmingSystem/Blueprints/Plants/BP_MasterPlant.BP_MasterPlant_C"))
  (for _array_element _outactors
    (bind _plantcomponent (Class|BPFarmingPlantInterface|PFSPlantComponent(Message) _array_element))
    (bind _output_get (LocalVariables|SetPlantComponentsL _plantcomponent))
    (if (not (Utilities|Array|ContainsItem (Variables|/Game/PlayerFarmingSystem/Blueprints/Components/BP_PlantComponent.BP_PlantComponent_C|GetWarmthZones _output_get) self))
      (Utilities|Array|AddUnique (Variables|/Game/PlayerFarmingSystem/Blueprints/Components/BP_PlantComponent.BP_PlantComponent_C|GetWarmthZones _output_get) self)
      (Default|UpdateWarmth (LocalVariables|GetPlantComponentsL))))
  (Collision|SetCollisionEnabled (Variables|Default|GetBox) "NoCollision"))

(event EventBeginPlay
  ;[1 1 1] If server bind update events and update any overlapping plants warmth values
  (Development|SetHiddeninGame (Variables|Default|GetBox) (not (Variables|WarmthZoneSettings|Debug|GetShowArea)) false)
  (Networking|SwitchHasAuthority
    (:Authority
      (|BindUpdateEvent)
      (Warmth|UpdateOverlappingPlantsWarmth))))

(event Custom|UpdateDetectors
  (params (Location :type Vector))
  (bind _box (Variables|Default|GetBox))
  ;[1 1 1] When plant is placed inside the warmth zone, this runs to add warmth effect to that new plant
  (if (Class|KismetMathLibrary|IsPointinBoxwithTransform Location (Transformation|GetWorldTransform _box) (Components|Box|GetUnscaledBoxExtent _box))
    (Utilities|FlowControl|Delay (Math|Random|RandomFloatinRange 0.0 0.1))
    (Warmth|UpdateOverlappingPlantsWarmth)))

(fn PFSWarmthEffect
  (return (Variables|WarmthZoneSettings|Warmth|GetEnabled) (Variables|WarmthZoneSettings|Warmth|GetWarmth)))