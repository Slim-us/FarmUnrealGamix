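; BP_IconMaker is an editor-side actor in the farming system that bakes icon textures from its own scene capture view of a static or skeletal mesh.
; The construction script adds the actor to the capture's show-only list.
; BaketoRenderTexture draws an icon material into a render target, then saves it as a named, mipmap-free UI texture through an editor-only call.
; Reset restores mesh, light and capture transforms, plus directional light intensity.
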(event Custom|Bake%20to%20Render%20Texture
  ;[1 1 1] Creates textures using the camer view of the icon maker
  (Rendering|ClearRenderTarget2D (Variables|Texture|GetRenderTextureSample))
  (Rendering|DrawMaterialtoRenderTarget (Variables|Texture|GetRenderTextureSample) "/Game/PlayerFarmingSystem/Materials/M_RenderIconTexture.M_RenderIconTexture")
  (bind _returnvalue (Class|KismetRenderingLibrary|RenderTargetCreateStaticTexture2DEditorOnly (Variables|Texture|GetRenderTextureSample) (Variables|Texture|GetTextureName) "TC_Default" "TMGS_NoMipmaps"))
  (Variables|/Script/Engine.Texture|SetLODGroup _returnvalue "TEXTUREGROUP_UI"))

(event Custom|Reset
  ;[1 1 1] Resets all the locations, rotation and light intensity
  (Transformation|ResetRelativeTransform (Variables|Default|GetStaticMesh))
  (Transformation|SetRelativeTransform (Variables|Default|GetDirectionalLight) (Math|Transform|MakeTransform "0, 0,100.000000" "0, 0, 0" "1,1,1") false false)
  (Transformation|SetRelativeTransform (Variables|Default|GetSkyLight) (Math|Transform|MakeTransform "0, 0,50.000000" "0, 0, 0" "1,1,1") false false)
  (Transformation|SetRelativeTransform (Variables|Default|GetSceneCaptureComponent2D) (Math|Transform|MakeTransform "-30.000000, 0,0.000000" "0, 0, 0" "1,1,1") false false)
  (Rendering|Components|Light|SetIntensity (Variables|Default|GetDirectionalLight) 5.0))

(fn ConstructionScript
  (Utilities|Array|Add (Variables|/Script/Engine.SceneCaptureComponent|GetShowOnlyActors (Variables|Default|GetSceneCaptureComponent2D)) self))