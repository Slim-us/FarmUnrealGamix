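; Game mode component for the farming system that holds shared day/night and rain state.
; On begin play it caches all directional lights in the level as sun lights for later use.
; Setters update night, rain and rain amount only when values change, then fire event dispatchers to notify other actors.
; Debug mode prints each state change on screen.
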(fn SetAllDirectionalLights
  ;[1 1 1] Get directional lights (Sun lights and store for use later)
  (bind _outactors (Actor|GetAllActorsOfClass "/Script/Engine.DirectionalLight"))
  (Variables|DoNotEdit|SetDirectionalLights _outactors))

(fn SetIsNight
  (params (IsNight :type Boolean))
  (if (not (Math|Boolean|Equal(Boolean) IsNight (Variables|TimeOfDay|GetIsNight)))
    ;[1 1 1] Set is night and call event dispatecher on other actors
    (bind _output_get (Variables|TimeOfDay|SetIsNight IsNight))
    (Default|CallUpdateIsNight _output_get)
    ;[1 1 1] Debug text
    (Development|PrintString (Utilities|String|SelectString "Night" "Day" (Variables|TimeOfDay|GetIsNight)) (Variables|Debug|GetDebugMode) true "(R=0.000000,G=1.000000,B=0.000000,A=1.000000)" 3.0)))

(fn SetIsRaining
  (params (IsRaining :type Boolean) (RainAmount :type Float%20%28single-precision%29))
  ;[1 1 1] Set is raining and rain amoun, then call event dispatcher on other actors
  (if (not (and (Math|Boolean|Equal(Boolean) IsRaining (Variables|Weather|GetIsRaining)) (== RainAmount (Variables|Weather|GetRainAmount))))
    (Variables|Weather|SetIsRaining IsRaining)
    (Variables|Weather|SetRainAmount RainAmount)
    (Default|CallUpdateIsRaining (Variables|Weather|GetIsRaining) (Variables|Weather|GetRainAmount))
    ;[1 1 1] Debug text
    (Development|PrintString (Utilities|String|SelectString "Raining" "Dry" (Variables|Weather|GetIsRaining)) (Variables|Debug|GetDebugMode) true "(R=0.000000,G=1.000000,B=0.000000,A=1.000000)" 3.0)))

(event EventBeginPlay
  ;[1 1 1] On begin play set direction lights
  (Lights|SetAllDirectionalLights))