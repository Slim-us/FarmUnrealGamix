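; Warmth source scene component for the farming system that registers itself with nearby warmth detectors, by default only those on plants.
; A sphere overlap within its warmth radius finds detector components, adds itself to their sources and tells newly registered plants to update warmth.
; It scans on server BeginPlay, skipping preview owners, and rescans after a short random delay when a game mode update event reports a location within range.
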(fn UpdateSurroundingWarmthDetectors
  ;[1 1 1] Get all actors within radius only plants if only detect plants true (Default is true)
  (bind _outactors (Collision|SphereOverlapActors (Transformation|GetWorldLocation) (Variables|WarmthSourceSettings|GetWarmthRadius) (Utilities|Array|MakeArray "ObjectTypeQuery2") (select (Variables|WarmthSourceSettings|GetOnlyDetectPlants) "/Game/PlayerFarmingSystem/Blueprints/Plants/BP_MasterPlant.BP_MasterPlant_C" 0)))
  (bind _output_get (LocalVariables|SetPlantActorsL _outactors))
  ;[1 1 1] Check if the actors have a warmth detector and add self to warmth detect's sources
  (for _array_element _output_get
    (LocalVariables|SetPlantL _array_element)
    (bind _output_get_2 (LocalVariables|SetWarmthDetectorL (Actor|GetComponentbyClass _array_element "/Game/PlayerFarmingSystem/Blueprints/Components/BP_WarmthDetectorComponent.BP_WarmthDetectorComponent_C")))
    (Utilities|IsValid _output_get_2
      (:Is%20Valid
        (if (not (Utilities|Array|ContainsItem (Variables|/Game/PlayerFarmingSystem/Blueprints/Components/BP_WarmthDetectorComponent.BP_WarmthDetectorComponent_C|GetWarmthSources _output_get_2) self))
          (Utilities|Array|AddUnique (Variables|/Game/PlayerFarmingSystem/Blueprints/Components/BP_WarmthDetectorComponent.BP_WarmthDetectorComponent_C|GetWarmthSources (LocalVariables|GetWarmthDetectorL)) self)
          ;[1 1 1] Update plant warmth value
          (bind _plantcomponent (Class|BPFarmingPlantInterface|PFSPlantComponent(Message) (LocalVariables|GetPlantL)))
          (Default|UpdateWarmth _plantcomponent))))))

(event EventBeginPlay
  ;[1 1 1] On begin play if server and not attached to a preview bind update events and update near by warmth detectors
  (Utilities|IsServer?
    (:true
      (Utilities|FlowControl|Delay 0.0)
      (Utilities|IsPreview?
        (:false
          (|BindUpdateEvent)
          (Warmth|UpdateSurroundingWarmthDetectors))))))

(event Custom|UpdateDetectors
  (params (Location :type Vector))
  ;[1 1 1] When near provided location update near by light detectors
  (if (<= (Math|Vector|Distance(Vector) Location (Transformation|GetWorldLocation)) (Variables|WarmthSourceSettings|GetWarmthRadius))
    (Utilities|FlowControl|Delay (Math|Random|RandomFloatinRange 0.0 0.1))
    (Warmth|UpdateSurroundingWarmthDetectors)))