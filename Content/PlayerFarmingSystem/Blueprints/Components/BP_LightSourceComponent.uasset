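; Scene component that marks its owner as a light source for nearby plants in the farming system.
; On the server, for non-preview owners, it sphere-overlaps plants within its light radius and adds itself to each light detector component's source list.
; It binds to the farming game mode component's update event and rescans when the broadcast location is within range, after a small random delay.
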(fn UpdateSurroundingLightDetectors
  ;[1 1 1] Get all plant actors in the radius
  (bind _outactors (Collision|SphereOverlapActors (Transformation|GetWorldLocation) (Variables|LightSourceSettings|GetLightRadius) (Utilities|Array|MakeArray "ObjectTypeQuery2") "/Game/PlayerFarmingSystem/Blueprints/Plants/BP_MasterPlant.BP_MasterPlant_C"))
  (bind _output_get (LocalVariables|SetPlantActorsL _outactors))
  ;[1 1 1] Loop though the plant's light detector components and add this light source to there light sources array
  (for _array_element _output_get
    (bind _output_get_2 (LocalVariables|SetLightDetectorL (Actor|GetComponentbyClass _array_element "/Game/PlayerFarmingSystem/Blueprints/Components/BP_LightDetectorComponent.BP_LightDetectorComponent_C")))
    (Utilities|IsValid _output_get_2
      (:Is%20Valid
        (if (not (Utilities|Array|ContainsItem (Variables|/Game/PlayerFarmingSystem/Blueprints/Components/BP_LightDetectorComponent.BP_LightDetectorComponent_C|GetLightSources _output_get_2) self))
          (Utilities|Array|AddUnique (Variables|/Game/PlayerFarmingSystem/Blueprints/Components/BP_LightDetectorComponent.BP_LightDetectorComponent_C|GetLightSources (LocalVariables|GetLightDetectorL)) self))))))

(event EventBeginPlay
  ;[1 1 1] On begin play if server and not attached to a preview bind update events and update near by light detectors
  (Utilities|IsServer?
    (:true
      (Utilities|FlowControl|Delay 0.0)
      (Utilities|IsPreview?
        (:False
          (|BindUpdateEvent)
          (Light|UpdateSurroundingLightDetectors))))))

(event Custom|UpdateDetectors
  (params (Location :type Vector))
  ;[1 1 1] When near provided location update near by light detectors
  (if (<= (Math|Vector|Distance(Vector) Location (Transformation|GetWorldLocation)) (Variables|LightSourceSettings|GetLightRadius))
    (Utilities|FlowControl|Delay (Math|Random|RandomFloatinRange 0.0 0.1))
    (Light|UpdateSurroundingLightDetectors)))