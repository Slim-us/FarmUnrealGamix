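; Sprinkler source component for the player farming system that waters nearby plants while switched on.
; Toggling it broadcasts the new state and starts or clears a looping timer that calls AddWater.
; Each tick sphere-overlaps plant actors within a radius, skips previews and plants that don't use water, then increases water on their plant components.
; An optional line trace withholds water from plants blocked from the sprinkler.
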(fn StartAddWaterTimer
  ;[1 1 1] If not already running start add water timer
  (if (not (Utilities|Time|IsValidTimerHandle (Variables|DoNotEdit|GetWaterAddTimer)))
    (bind _returnvalue (Utilities|Time|SetTimerbyFunctionName 0 "AddWater" (Variables|SprinklerSettings|Water|GetWaterAddTime) true 0.0 0.1))
    (Variables|DoNotEdit|SetWaterAddTimer _returnvalue)))

(fn UpdateSprinkleron
  (params (SprinklerOn :type Boolean))
  ;[1 1 1] Sets the sprinkler on/off and starts the add water timer
  (bind _output_get (Variables|SprinklerSettings|SetSprinklerOn SprinklerOn))
  (Default|CallSprinkleronUpdated _output_get)
  (Utilities|SprinklerOn?
    (:true
      (Timer|StartAddWaterTimer))
    (:false
      (Utilities|Time|ClearandInvalidateTimerbyHandle (Variables|DoNotEdit|GetWaterAddTimer)))))

(fn AddWater
  ;[1 1 1] Check if sprinkler on, get all plant actors within radius and loop though results
  (if (Variables|SprinklerSettings|GetSprinklerOn)
    (bind (_outactors _returnvalue) (Collision|SphereOverlapActors (Transformation|GetWorldLocation) (Variables|SprinklerSettings|Water|GetWaterAddRadius) (Utilities|Array|MakeArray "ObjectTypeQuery2") "/Game/PlayerFarmingSystem/Blueprints/Plants/BP_MasterPlant.BP_MasterPlant_C" (Utilities|Array|MakeArray (Components|GetOwner))))
    (if _returnvalue
      (bind _output_get (LocalVariables|SetPlantsL _outactors))
      (for _array_element _output_get
        (LocalVariables|SetPlantL _array_element)
        ;[1 1 1] Check plant isnt preview and get plant component
        (bind _preview (Class|BPFarmingPlacementInterface|PFSGetPreview(Message) (LocalVariables|GetPlantL)))
        (if (not _preview)
          (bind _plantcomponent (Class|BPFarmingPlantInterface|PFSPlantComponent(Message) (LocalVariables|GetPlantL)))
          (bind _output_get_2 (LocalVariables|SetPlantComponentL _plantcomponent))
          (Utilities|IsValid _output_get_2
            (:Is%20Valid
              ;[1 1 1] Check plant uses water
              (if (Variables|/Game/PlayerFarmingSystem/Blueprints/Components/BP_PlantComponent.BP_PlantComponent_C|GetUseWater (LocalVariables|GetPlantComponentL))
                ;[1 1 1] Check plant has line of sight to the sprinkler
                (if (Variables|SprinklerSettings|Collision|GetUseBlockingTraceCheck)
                  (bind (_outhit _returnvalue_2) (Collision|LineTraceByChannel (Transformation|GetWorldLocation) (.Origin (Collision|GetActorBounds (LocalVariables|GetPlantL) false false)) (Variables|SprinklerSettings|Collision|GetBlockTraceChannel) false (Utilities|Array|MakeArray (Components|GetOwner)) (Variables|SprinklerSettings|Debug|GetBlockTraceDebug) true "(R=1.000000,G=0.000000,B=0.000000,A=1.000000)" "(R=0.000000,G=1.000000,B=0.000000,A=1.000000)" 1.0))
                  (if _returnvalue_2
                    (if (== (.HitActor (Collision|BreakHitResult _outhit)) (LocalVariables|GetPlantL))
                      ;[1 1 1] Increase plant water
                      (Default|IncreaseWater (LocalVariables|GetPlantComponentL) (Variables|SprinklerSettings|Water|GetWaterAddAmount) :!label _label))
                    (else
                      (goto _label)))
                  (else
                    ;[1 1 1] Increase plants water
                    (Default|IncreaseWater (LocalVariables|GetPlantComponentL) (Variables|SprinklerSettings|Water|GetWaterAddAmount))))))))))
    (else
      (Utilities|Time|ClearandInvalidateTimerbyHandle (Variables|DoNotEdit|GetWaterAddTimer)))))