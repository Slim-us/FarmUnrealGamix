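; Scene component in the farming system that detects how much light reaches its owner.
; LightAmount first sets HasDirectionalLight by the selected mode: always true, an upward trace, or traces along each directional light from the GameMode.
; It then sums enabled entries in LightSources, optionally requiring line of sight, prunes invalid ones and returns a total capped at 100.
; Debug mode draws traces and reports what blocks directional light.
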(fn BasicDirectionalLightCheck
  (bind _returnvalue (Transformation|GetWorldLocation))
  ;[1 1 1] Basic directional light detector, just does a line trace up, if it does not hit anything then directional light (sun light) is true
  (bind (_outhit _returnvalue_2) (Collision|LineTraceByChannel _returnvalue (+ _returnvalue (Math|Vector|MakeVector 0.0 0.0 (Variables|DetectionSettings|Collision|GetBasicCheckDistance))) (Variables|DetectionSettings|Collision|GetLightCollisionChannel) false (Utilities|Array|MakeArray (Components|GetOwner) (Actor|GetAttachParentActor (Components|GetOwner))) (select (Variables|DetectionSettings|Debug|GetDebugMode) "ForDuration" "None") true "(R=1.000000,G=0.000000,B=0.000000,A=1.000000)" "(R=0.000000,G=1.000000,B=0.000000,A=1.000000)" 0.5))
  (if _returnvalue_2
    (Variables|DoNotEdit|SetHasDirectionalLight false)
    (Debug|DebugText (Utilities|String|Append "\"" (Utilities|GetDisplayName (.HitActor (Collision|BreakHitResult _outhit))) "\" is blocking the light to " "\"" (Utilities|GetDisplayName (Components|GetOwner)) "\"") "(R=1.000000,G=0.000000,B=0.000000,A=1.000000)" 2.0)
    (else
      (Variables|DoNotEdit|SetHasDirectionalLight true)
      (return))))

(fn AdvancedDirectionalLightCheck
  ;[1 1 1] Get directional lights from game mode and location
  (bind _directionallights (Class|BPFarmingGameModeInterface|PFSGetDirectionalLights(Message) (Game|GetGameMode)))
  (Variables|DoNotEdit|SetDirectionalLights _directionallights)
  (LocalVariables|SetComponentLocationL (Transformation|GetWorldLocation))
  ;[1 1 1] Line trace to the direction light location, if line traces doesnt hit any thing then directional light is true
  (for _array_element (Variables|DoNotEdit|GetDirectionalLights)
    (bind (_outhit _returnvalue) (Collision|LineTraceByChannel (+ (LocalVariables|GetComponentLocationL) (* (Math|Rotator|GetRotationXVector (Transformation|GetActorRotation _array_element)) (* (Variables|DetectionSettings|Collision|GetAdvancedCheckDistance) -1.0))) (LocalVariables|GetComponentLocationL) (Variables|DetectionSettings|Collision|GetLightCollisionChannel) false (Utilities|Array|MakeArray (Components|GetOwner) (Actor|GetAttachParentActor (Components|GetOwner))) (select (Variables|DetectionSettings|Debug|GetDebugMode) "ForDuration" "None") true "(R=1.000000,G=0.000000,B=0.000000,A=1.000000)" "(R=0.000000,G=1.000000,B=0.000000,A=1.000000)" 0.5))
    (if _returnvalue
      (Debug|DebugText (Utilities|String|Append "\"" (Utilities|GetDisplayName (.HitActor (Collision|BreakHitResult _outhit))) "\" is blocking the light to " "\"" (Utilities|GetDisplayName (Components|GetOwner)) "\"") "(R=1.000000,G=0.000000,B=0.000000,A=1.000000)" 2.0)
      (else
        (Variables|DoNotEdit|SetHasDirectionalLight true)
        (return))))
  (Variables|DoNotEdit|SetHasDirectionalLight false))

(fn DebugText
  (params (InString :type String) (TextColor :type Linear%20Color%20Structure :default "(R=0.000000,G=1.000000,B=0.000000,A=1.000000)") (Duration :type Float%20%28double-precision%29))
  (bind _debugmode (Variables|DetectionSettings|Debug|GetDebugMode))
  ;[1 1 1] Debug text shows if Debug Mode is true
  (Development|PrintString InString _debugmode _debugmode TextColor Duration))

(fn LightAmount
  ;[1 1 1] Switch depending on detection type
  (switch Utilities|FlowControl|Switch|SwitchonE_LightDetectType (Variables|DetectionSettings|GetDirectionalLightDetectionType)
    (:NewEnumerator2
      (Variables|DoNotEdit|SetHasDirectionalLight true))
    (:NewEnumerator0
      (Checks|AdvancedDirectionalLightCheck))
    (:NewEnumerator1
      (Checks|BasicDirectionalLightCheck)))
  ;[1 1 1] Loop though all near by light sources
  (for _array_element (Variables|DoNotEdit|GetLightSources)
    (bind _output_get (LocalVariables|SetLightSourceL _array_element))
    (Utilities|IsValid _output_get
      (:Is%20Valid
        ;[1 1 1] Check the light source is set to enabled, then do a line trace to make sure nothing blocks the light, if total light amount hits 100 end the function.
        (if (Variables|/Game/PlayerFarmingSystem/Blueprints/Components/BP_LightSourceComponent.BP_LightSourceComponent_C|GetEnabled (LocalVariables|GetLightSourceL))
          (if (Variables|DetectionSettings|GetUseLineOfSightDetectionForLightSources)
            (bind _returnvalue (Collision|LineTraceByChannel (Transformation|GetWorldLocation) (Transformation|GetWorldLocation (LocalVariables|GetLightSourceL)) (Variables|DetectionSettings|Collision|GetLightCollisionChannel) false (Utilities|Array|MakeArray (Components|GetOwner) (Components|GetOwner (LocalVariables|GetLightSourceL))) (select (Variables|DetectionSettings|Debug|GetDebugMode) "ForDuration" "None")))
            (if (not _returnvalue)
              (bind _output_get_2 (LocalVariables|SetLightAmountL (+ (LocalVariables|GetLightAmountL) (Variables|/Game/PlayerFarmingSystem/Blueprints/Components/BP_LightSourceComponent.BP_LightSourceComponent_C|GetLightAmount (LocalVariables|GetLightSourceL))) :!label _label))
              (if (>= _output_get_2 1e+02)
                (return 1e+02)))
            (else
              (goto _label)))))
      (:Is%20Not%20Valid
        (Utilities|Array|RemoveItem (Variables|DoNotEdit|GetLightSources) (LocalVariables|GetLightSourceL)))))
  (return (Math|Float|Clamp(Float) (LocalVariables|GetLightAmountL) 0.0 1e+02)))