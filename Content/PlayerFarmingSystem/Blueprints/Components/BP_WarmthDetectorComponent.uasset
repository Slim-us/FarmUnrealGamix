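; Warmth detector component for the player farming system that reports how much warmth reaches its location, from 0 to 100.
; WarmthAmount sums enabled sources in WarmthSources that have an unblocked line trace on the warmth collision channel, stopping early at the cap and removing invalid entries.
; BeginPlay caches the farming game mode component through an interface message.
; Debug Mode toggles trace drawing and the DebugText print helper.
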(fn DebugText
  (params (InString :type String) (TextColor :type Linear%20Color%20Structure :default "(R=0.000000,G=1.000000,B=0.000000,A=1.000000)") (Duration :type Float%20%28double-precision%29))
  (bind _debugmode (Variables|DetectionSettings|Debug|GetDebugMode))
  ;[1 1 1] Debug text shows if Debug Mode is true
  (Development|PrintString InString _debugmode _debugmode TextColor Duration))

(fn WarmthAmount
  ;[1 1 1] Loop though all near by light sources
  (for _array_element (Variables|DoNotEdit|GetWarmthSources)
    (bind _output_get (LocalVariables|SetWarmthSourceL _array_element))
    (Utilities|IsValid _output_get
      (:Is%20Valid
        ;[1 1 1] Check the light source is set to enabled, then do a line trace to make sure nothing blocks the light, if total light amount hits 100 end the function.
        (if (Variables|/Game/PlayerFarmingSystem/Blueprints/Components/BP_WarmthSourceComponent.BP_WarmthSourceComponent_C|GetEnabled (LocalVariables|GetWarmthSourceL))
          (bind _returnvalue (Collision|LineTraceByChannel (Transformation|GetWorldLocation) (Transformation|GetWorldLocation (LocalVariables|GetWarmthSourceL)) (Variables|DetectionSettings|Collision|GetWarmthCollisionChannel) false (Utilities|Array|MakeArray (Components|GetOwner) (Components|GetOwner (LocalVariables|GetWarmthSourceL))) (select (Variables|DetectionSettings|Debug|GetDebugMode) "ForDuration" "None") true "(R=1.000000,G=0.000000,B=0.000000,A=1.000000)" "(R=0.000000,G=1.000000,B=0.000000,A=1.000000)" 2.0))
          (if (not _returnvalue)
            (bind _output_get_2 (LocalVariables|SetWarmthAmountL (+ (LocalVariables|GetWarmthAmountL) (Variables|/Game/PlayerFarmingSystem/Blueprints/Components/BP_WarmthSourceComponent.BP_WarmthSourceComponent_C|GetWarmthAmount (LocalVariables|GetWarmthSourceL)))))
            (if (>= _output_get_2 1e+02)
              (return 1e+02)))))
      (:Is%20Not%20Valid
        (Utilities|Array|RemoveItem (Variables|DoNotEdit|GetWarmthSources) (LocalVariables|GetWarmthSourceL)))))
  (return (Math|Float|Clamp(Float) (LocalVariables|GetWarmthAmountL) 0.0 1e+02)))

(event EventBeginPlay
  ;[1 1 1] Set reference to gamemode component
  (bind _farminggamemodecomponent (Class|BPFarmingGameModeInterface|PFSGetFarmingGameModeComponent(Message) (Game|GetGameMode)))
  (Variables|Default|SetFarmingGamemodeComponent _farminggamemodecomponent))