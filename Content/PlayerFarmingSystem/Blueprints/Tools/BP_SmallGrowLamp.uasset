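; BP_SmallGrowLamp is a small grow lamp tool in the player farming system, built as a child of a parent Blueprint.
; Its ToggleLightComponents override calls the parent, then switches the glass look through a dynamic material instance of M_Light and its SwitchedOn scalar parameter.
; AddDestructionMesh adds a Geometry Collection component to serve as the lamp's destruction mesh.
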(fn ConstructionScript
  (|CallParentFunction))

(fn ToggleLightComponents
  (params (bNewVisibility :type Boolean))
  (|CallParentFunction bNewVisibility)
  ;[1 0 0] Sets on/off glass material (You can remove this if you duplicated this blueprint)
  (bind _returnvalue (Rendering|Material|CreateDynamicMaterialInstance (Variables|Default|GetSM_SmallGrowLightGlass) 0 "/Game/PlayerFarmingSystem/Materials/M_Light.M_Light" "None" :!class /Script/Engine.PrimitiveComponent))
  (Utilities|IsValid _returnvalue
    (:Is%20Valid
      (Rendering|Material|SetScalarParameterValue _returnvalue "SwitchedOn" (Math|Float|SelectFloat 1.0 0.0 bNewVisibility) :!class /Script/Engine.MaterialInstanceDynamic))))

(fn AddDestructionMesh
  ;[1 1 1] Destruction mesh spawned
  (AddComponent|AddGeometryCollectionComponent false (Math|Transform|MakeTransform "0, 0, 0")))