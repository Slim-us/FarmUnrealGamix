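; Base grow light tool for the player farming system that can be toggled by interaction and acts as a light and warmth source.
; BeginPlay gathers its light and source components, and the LightOn RepNotify updates light visibility, enabling light and warmth sources only on authority.
; Previews stay unlit, while placed lights follow StartWithLightOn and save class, transform and on state into the current level's save data.
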(fn ConstructionScript
  (|CallParentFunction))

(fn OnRepLighton
  ;[1 1 1] Runs when you change the LightOn variable, then updates the light components to be on/off
  (Lights|UpdateLighton))

(fn UpdateLighton
  (Utilities|FlowControl|Sequence
    (:then_0
      ;[1 1 1] Turns lights on and off
      (if (Variables|LightSettings|GetLightOn)
        (Lights|ToggleLightComponents true)
        (else
          (Lights|ToggleLightComponents false))))
    (:then_1
      ;[1 1 1] Turns light source components on and off
      (Networking|SwitchHasAuthority
        (:Authority
          (Utilities|FlowControl|Sequence
            (:then_0
              (for _array_element (Variables|DoNotEdit|GetLightSources)
                (Variables|/Game/PlayerFarmingSystem/Blueprints/Components/BP_LightSourceComponent.BP_LightSourceComponent_C|SetEnabled _array_element (Variables|LightSettings|GetLightOn))))
            (:then_1
              (for _array_element_2 (Variables|DoNotEdit|GetWarmthSources)
                (Variables|/Game/PlayerFarmingSystem/Blueprints/Components/BP_WarmthSourceComponent.BP_WarmthSourceComponent_C|SetEnabled _array_element_2 (Variables|LightSettings|GetLightOn))))))))))

(fn ToggleLight
  ;[1 1 1] If light on set to off, if off set to on
  (Variables|LightSettings|SetLightOn (select (Variables|LightSettings|GetLightOn) false true)))

(fn ToggleLightComponents
  (params (bNewVisibility :type Boolean))
  ;[1 1 1] Sets visibility of all light components
  (Rendering|SetVisibility (Variables|DoNotEdit|GetLights) bNewVisibility false))

(fn SetToolSaveData
  ;[1 1 1] Sets the light stats to the ToolSaveData struct
  (return (Utilities|Struct|MakeS_ToolSaveData (Utilities|GetClass self) (Transformation|GetActorTransform) (Variables|LightSettings|GetLightOn))))

(fn SaveLightData
  (params (SaveData :type BP%20Farming%20Save%20Object%20Object%20Reference))
  ;[1 1 1] Gets the current level save data
  (bind _returnvalue (Game|GetCurrentLevelName true))
  (bind _levelsavedata (Default|CurrentLevelSaveData SaveData _returnvalue))
  (LocalVariables|SetLevelSaveDataL _levelsavedata)
  ;[1 1 1] Sets the lights class, location and on/off state
  (bind _toolsavedata (Saving|SetToolSaveData))
  (LocalVariables|SetLightSaveDataL _toolsavedata)
  ;[1 1 1] Adds light data to the level save data
  (Utilities|Array|Add (Utilities|Struct|BreakS_LevelSaveData (LocalVariables|GetLevelSaveDataL)) (LocalVariables|GetLightSaveDataL))
  ;[1 1 1] Updates level save data in the save object
  (Default|UpdateLevelSaveData SaveData (LocalVariables|GetLevelSaveDataL)))

(fn DestructionEffect
  (for _array_element (Variables|DoNotEdit|GetLights)
    (Components|DestroyComponent _array_element))
  (for _array_element_2 (Variables|DoNotEdit|GetLightSources)
    (Components|DestroyComponent _array_element_2))
  (for _array_element_3 (Variables|DoNotEdit|GetWarmthSources)
    (Components|DestroyComponent _array_element_3)))

(event EventPFSSetPreview
  (params (Preview :type Boolean))
  ;[1 1 1] On SetPreview check if preview, if is set light off, if not check if start with light on and set light on or off
  (|CallParentFunction Preview)
  (Utilities|IsPreview?
    (:true
      (Variables|LightSettings|SetLightOn false))
    (:false
      (if (Variables|LightSettings|GetStartWithLightOn)
        (Variables|LightSettings|SetLightOn true)
        (else
          (Variables|LightSettings|SetLightOn false))))))

(event EventBeginPlay
  ;[1 1 1] On Begin Play set references to source components and lights, if not preview update light on state
  (|CallParentFunction)
  (Variables|DoNotEdit|SetLights (Actor|GetComponentsByClass "/Script/Engine.LightComponent"))
  (Variables|DoNotEdit|SetLightSources (Actor|GetComponentsByClass "/Game/PlayerFarmingSystem/Blueprints/Components/BP_LightSourceComponent.BP_LightSourceComponent_C"))
  (Variables|DoNotEdit|SetWarmthSources (Actor|GetComponentsByClass "/Game/PlayerFarmingSystem/Blueprints/Components/BP_WarmthSourceComponent.BP_WarmthSourceComponent_C"))
  (Utilities|IsPreview?
    (:false
      (Lights|UpdateLighton))))

(event EventPFSSaveActor
  (params (SaveObject :type BP%20Farming%20Save%20Object%20Object%20Reference))
  ;[1 1 1] Runs when the game saves, to store the plants data in the save game object
  (Utilities|IsPreview?
    (:false
      (Saving|SaveLightData SaveObject))))

(event EventPFSToggleOn/Off
  (params (Enabled :type Boolean))
  ;[1 1 1] Toggles light on or off
  (Variables|LightSettings|SetLightOn Enabled))

(event EventPFSInteract
  (params (KeyDown :type Boolean) (PlayerFarmingComponent :type BP%20Player%20Farming%20Component%20Object%20Reference))
  ;[1 1 1] On Interact check if key down and if true toggle light on or off
  (if KeyDown
    (Lights|ToggleLight)))