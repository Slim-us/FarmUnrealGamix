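; Base sprinkler tool for the farming system that players toggle on or off by interacting, with child classes supplying the effect.
; The SprinklerOn RepNotify calls the overridable SprinklerEffect and, on authority only, passes the state to every sprinkler source component.
; Preview placements stay off and are not saved, while placed sprinklers take their configured start state and save class, transform and state to the level's save data.
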(fn ConstructionScript
  (|CallParentFunction))

(fn OnRepSprinkleron
  ;[1 1 1] If sprinkler stat changes update if On
  (Update|UpdateSprinkleron))

(fn SprinklerEffect
  ;[1 1 1] Overriden in children
)

(fn UpdateSprinkleron
  (Utilities|FlowControl|Sequence
    (:then_0
      ;[1 1 1] Call effect code in child
      (Effects|SprinklerEffect))
    (:then_1
      ;[1 1 1] Toggles on/off the sprinkler components
      (Networking|SwitchHasAuthority
        (:Authority
          (for _array_element (Variables|DoNotEdit|GetSprinklerSourceComponents)
            (Default|UpdateSprinkleron _array_element (Variables|SprinklerSettings|GetSprinklerOn))))))))

(fn SaveSprinklerData
  (params (SaveData :type BP%20Farming%20Save%20Object%20Object%20Reference))
  ;[1 1 1] Get current level's save data
  (bind _returnvalue (Game|GetCurrentLevelName true))
  (bind _levelsavedata (Default|CurrentLevelSaveData SaveData _returnvalue))
  (LocalVariables|SetLevelSaveDataL _levelsavedata)
  ;[1 1 1] Set sprinkler class, location and if on or off
  (Utilities|Struct|SetmembersinS_ToolSaveData (LocalVariables|GetSprinklerSaveDataL) (Utilities|GetClass self) (Transformation|GetActorTransform) (Variables|SprinklerSettings|GetSprinklerOn))
  ;[1 1 1] Add data to the level save data
  (Utilities|Array|Add (Utilities|Struct|BreakS_LevelSaveData (LocalVariables|GetLevelSaveDataL)) (LocalVariables|GetSprinklerSaveDataL))
  ;[1 1 1] Update save data objects level data
  (Default|UpdateLevelSaveData SaveData (LocalVariables|GetLevelSaveDataL)))

(fn ToggleSprinkler
  ;[1 1 1] If on turns off, if off turns on
  (Variables|SprinklerSettings|SetSprinklerOn (select (Variables|SprinklerSettings|GetSprinklerOn) false true)))

(fn SetToolSaveData
  ;[1 1 1] Sets the sprinkler stats to the ToolSaveData struct
  (return (Utilities|Struct|MakeS_ToolSaveData (Utilities|GetClass self) (Transformation|GetActorTransform) (Variables|SprinklerSettings|GetSprinklerOn))))

(fn DestructionEffect
  (|CallParentFunction)
  (Components|Activation|Deactivate (Actor|GetComponentsByClass "/Script/Engine.ParticleSystemComponent")))

(event EventBeginPlay
  ;[1 1 1] On Begin play set reference to source components and if not preview update if On
  (|CallParentFunction)
  (Variables|DoNotEdit|SetSprinklerSourceComponents (Actor|GetComponentsByClass "/Game/PlayerFarmingSystem/Blueprints/Components/BP_SprinklerSourceComponent.BP_SprinklerSourceComponent_C"))
  (Utilities|IsPreview?
    (:false
      (Update|UpdateSprinkleron))))

(event EventPFSSetPreview
  (params (Preview :type Boolean))
  ;[1 1 1] On SetPreview check if is preview, if is set off, if not preview check if should start on and set On or Off
  (|CallParentFunction Preview)
  (Utilities|IsPreview?
    (:true
      (Variables|SprinklerSettings|SetSprinklerOn false))
    (:false
      (if (Variables|SprinklerSettings|GetStartWithSprinklerOn)
        (Variables|SprinklerSettings|SetSprinklerOn true)
        (else
          (Variables|SprinklerSettings|SetSprinklerOn false))))))

(event EventPFSToggleOn/Off
  (params (Enabled :type Boolean))
  ;[1 1 1] On ToggleOn/Off set if On or Off
  (Variables|SprinklerSettings|SetSprinklerOn Enabled))

(event EventPFSInteract
  (params (KeyDown :type Boolean) (PlayerFarmingComponent :type BP%20Player%20Farming%20Component%20Object%20Reference))
  ;[1 1 1] On Interact if key down toggle sprinkler on or off
  (if KeyDown
    (Update|ToggleSprinkler)))

(event EventPFSSaveActor
  (params (SaveObject :type BP%20Farming%20Save%20Object%20Object%20Reference))
  ;[1 1 1] On SaveActor check not preview and if not save sprinkler data to save object
  (Utilities|IsPreview?
    (:false
      (Saving|SaveSprinklerData SaveObject))))