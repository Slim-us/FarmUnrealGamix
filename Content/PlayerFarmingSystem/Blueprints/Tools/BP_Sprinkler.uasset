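; Sprinkler for the player farming system, extending a parent class with the visual effect for its on and off state.
; When on, it activates the particle emitter and starts a looping timer that spins the head in small yaw steps scaled by RotateTime, avoiding Tick.
; When off, it stops the particles and clears the timer.
; It also provides a geometry collection component as its destruction mesh.
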(fn ConstructionScript
  (|CallParentFunction))

(fn SprinklerEffect
  (|CallParentFunction)
  (if (Variables|Default|GetSprinklerOn)
    (Components|Activation|Activate (Variables|Default|GetParticleEmitter) false)
    (Effects|StartTurnSprinklerTimer)
    (else
      (Components|Activation|Deactivate (Variables|Default|GetParticleEmitter))
      (Utilities|Time|ClearandInvalidateTimerbyHandle (Variables|DoNotEdit|GetTurnSprinklerTimer)))))

(fn TurnSprinkler
  (Transformation|SetRelativeRotation (Variables|Default|GetSprinklerHead) (Math|Rotator|CombineRotators (Variables|/Script/Engine.SceneComponent|GetRelativeRotation (Variables|Default|GetSprinklerHead)) (Math|Rotator|MakeRotator 0.0 0.0 (/ 15.0 (Variables|SprinklerSettings|GetRotateTime)))) false false))

(fn StartTurnSprinklerTimer
  (if (not (Utilities|Time|IsValidTimerHandle (Variables|DoNotEdit|GetTurnSprinklerTimer)))
    (bind _returnvalue (Utilities|Time|SetTimerbyFunctionName 0 "TurnSprinkler" 0.041 true 0.0 0.01))
    (Variables|DoNotEdit|SetTurnSprinklerTimer _returnvalue)))

(fn AddDestructionMesh
  ;[1 1 1] Destruction mesh spawned
  (AddComponent|AddGeometryCollectionComponent false (Math|Transform|MakeTransform "0, 0, 0")))