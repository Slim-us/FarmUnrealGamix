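; BP_MasterResourceBox is a base resource box for the player farming system that gives its configured resource to whoever interacts with it.
; On key-down interaction, CollectResource adds the resource type and amount through the player's PlayerFarmingComponent and sends a client notification with sound.
; An invalid component prints an error instead.
; The box does not destroy or deplete itself here, and its PFS widget function is empty.
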(fn ConstructionScript)

(fn CollectResource
  (params (PlayerFarmingComponent :type BP%20Player%20Farming%20Component%20Object%20Reference))
  (bind _resource (Variables|ResourceSettings|GetResource))
  (bind _resource_2 (Variables|ResourceSettings|GetResource))
  (bind (_resource_3 _amount) (Utilities|Struct|BreakS_Resources _resource))
  (bind (_resource_4 _amount_2) (Utilities|Struct|BreakS_Resources _resource_2))
  (Utilities|IsValid PlayerFarmingComponent
    (:Is%20Valid
      ;[1 1 1] Increase the resource amount of player
      (Default|IncreaseResource PlayerFarmingComponent _resource_4 _amount_2)
      ;[1 1 1] Creats notification for player that collected resource
      (Default|ClientCreateNotification PlayerFarmingComponent (Utilities|Struct|MakeS_NotificationDetails (Utilities|Text|FormatText "Collected {Item} ({Amount})" (Utilities|Text|ToText(Name) _resource_3) _amount) "(R=1.000000,G=1.000000,B=1.000000,A=1.000000)") true))
    (:Is%20Not%20Valid
      (Development|PrintString "ERROR :: PlayerFarmingComponent not valid when collecting resource from box" true true "(R=1.000000,G=0.000000,B=0.000000,A=1.000000)" 1e+01))))

(event EventPFSInteract
  (params (KeyDown :type Boolean) (PlayerFarmingComponent :type BP%20Player%20Farming%20Component%20Object%20Reference))
  ;[1 1 1] On Interact check key is down and run collect resources function
  (if KeyDown
    (CallFunction|CollectResource PlayerFarmingComponent)))

(fn PFSWidget
  (return 0))